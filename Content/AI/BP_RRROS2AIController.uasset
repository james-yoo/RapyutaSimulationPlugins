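; AI controller for a robot that picks up and drops payloads on ROS 2 commands.
; ROS 2 subscribers resolve locations or actor names, set targets and approach points, then set BTTask, which is also published as status.
; BT_ROS2Agent runs with pick and drop subtrees injected from PickDropParam; JSON general actions forward to the pawn.
; An older direct path chains AIMoveTo, linear moves, joint control and attach/detach through delegates.
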(event `self.ReceiveBeginPlay`
  (bind _returnvalue (`|AddComponentByClass` (`self.PickDropParamClass`)))
  (bind _output_get (set `self.PickDropParam` _returnvalue))
  (`/RapyutaSimulationPlugins/AI/BP_PickDropParam.CopyParam` _output_get (`self.DefaultPickDropParam`))
  (`self.BehaviorTreeSetting`))

(event `FindPickTargetpPyloadAndReachingPointEvent`
  (params (TargetPose :type "Vector Structure") (TargetPayload :type "Actor Object Reference"))
  (`self.FindTargetpayloadAndReachingPoint` TargetPose TargetPayload (`self.PayloadTag`)
    (:`Success`
      (set `self.FindTargetpayload` true))
    (:`Fail`
      (set `self.FindTargetpayload` false))))

(event `DropEvent`
  (params (DropLocation :type "Transform Structure") (TargetLocation :type "Actor Object Reference"))
  ;[1 1 1] legacy
  (bind _res (`self.PreDrop`))
  (if _res
    (`self.SetDropTarget` DropLocation TargetLocation)
    (bind _output_get (`self.FindDropReachingPoint` (`self.TargetLocation`)))
    (`self.DropImplEvent` _output_get)))

(event `DropImplEvent`
  (params (ReachintPoint :type "Transform Structure"))
  (bind (_returnvalue_x _returnvalue_y _returnvalue_z) (`KismetMathLibrary.BreakVector` (`self.K2_GetActorLocation`)))
  (bind _returnvalue (`self.K2_GetPawn`))
  (bind _location (.location ReachintPoint))
  ;[1 1 1] legacy
  (`|AIMoveTo` _returnvalue _location null 5.0 true
    (:`OnSuccess`
      (`self.LinearMoveToLocationWithDelegates` _returnvalue (`KismetMathLibrary.MakeVector` (.x _location) (.y _location) _returnvalue_z) (`KismetMathLibrary.MakeRotator` (.roll (.rotation ReachintPoint)) (.pitch (.rotation ReachintPoint)) (+ (.yaw (.rotation ReachintPoint)) 180.0)) (delegate `CustomEvent_14`) (delegate `CustomEvent_13`) 1.0 1.0 -1.0 (0.0 0.0 0.0) (`KismetMathLibrary.MakeRotator` 0.0)))
    (:`OnFail`
      (`self.PostDrop` false))))

(event `CustomEvent_7`
  ;[1 1 1] legacy
  (`self.AddLocalLinearMotionOffsetWthDelegates` (`self.K2_GetPawn`) (`KismetMathLibrary.MakeVector` (`/RapyutaSimulationPlugins/AI/BP_PickDropParam.DisToTarget` (`self.PickDropParam`))) (delegate `CustomEvent_11`) (delegate `CustomEvent_12`) :!label _label))

(event `CustomEvent_8`
  ;[1 1 1] legacy
  (`self.PostDrop` false))

(event `CustomEvent_11`
  (bind (_returnvalue_x _returnvalue_y _returnvalue_z) (`KismetMathLibrary.BreakVector` (`self.K2_GetActorLocation`)))
  (bind _attachmentjoint (`/RapyutaSimulationPlugins/AI/BP_PickDropParam.AttachmentJoint` (`self.PickDropParam`)))
  ;[1 1 1] legacy
  (`/Engine/EditorBlueprintResources/StandardMacros.IsValid` _attachmentjoint
    (:`Is Valid`
      (`RRJointComponent.SetSinglePositionTargetWithDelegates` _attachmentjoint (- (.z (.location (stale `DropImplEvent` ReachintPoint))) _returnvalue_z) (delegate `CustomEvent_18`) (delegate `CustomEvent_17`) -1.0 5.0))
    (:`Is Not Valid`
      (`self.K2_DetachFromActor` (`self.TargetPayload`) "KeepWorld" "KeepWorld" "KeepWorld" :!label _label_2)
      (`self.AddLocalLinearMotionOffsetWthDelegates` (`self.K2_GetPawn`) (`KismetMathLibrary.MakeVector` (* (`/RapyutaSimulationPlugins/AI/BP_PickDropParam.DisToTarget` (`self.PickDropParam`)) -1.0)) (delegate `CustomEvent_15`) (delegate `CustomEvent_16`)))))

(event `CustomEvent_12`
  ;[1 1 1] legacy
  (`self.PostDrop` false))

(event `CustomEvent_15`
  ;[1 1 1] legacy
  (`self.PostDrop` true))

(event `CustomEvent_16`
  ;[1 1 1] legacy
  (`self.PostDrop` false))

(event `CustomEvent_17`
  ;[1 1 1] legacy
  (`self.PostDrop` false))

(event `CustomEvent_18`
  ;[1 1 1] legacy
  (goto _label_2))

(event `CustomEvent_13`
  ;[1 1 1] legacy
  (`self.PostDrop` false))

(event `CustomEvent_14`
  (bind (_returnvalue_x _returnvalue_y _returnvalue_z) (`KismetMathLibrary.BreakVector` (`self.K2_GetActorLocation`)))
  (bind _attachmentjoint (`/RapyutaSimulationPlugins/AI/BP_PickDropParam.AttachmentJoint` (`self.PickDropParam`)))
  ;[1 1 1] legacy
  (`/Engine/EditorBlueprintResources/StandardMacros.IsValid` _attachmentjoint
    (:`Is Valid`
      (`RRJointComponent.SetSinglePositionTargetWithDelegates` _attachmentjoint (- (+ (.z (.location (stale `DropImplEvent` ReachintPoint))) (`/RapyutaSimulationPlugins/AI/BP_PickDropParam.PickOffset` (`self.PickDropParam`))) _returnvalue_z) (delegate `CustomEvent_7`) (delegate `CustomEvent_8`) -1.0 5.0))
    (:`Is Not Valid`
      (goto _label))))

(event `DropBTEvent`
  (params (DropLocation :type "Transform Structure") (TargetLocation :type "Actor Object Reference") (UseApproach :type Boolean) (ApproachLocation :type "Vector Structure") (ApproachLocationActor :type "Actor Object Reference") (UseDefaultApproach :type Boolean))
  (bind _res (`self.PreDrop`))
  (if _res
    (`self.SetDropTarget` DropLocation TargetLocation UseApproach ApproachLocation ApproachLocationActor UseDefaultApproach)
    (set `self.BTTask` "NewEnumerator1")))

(event `PickEvent`
  (params (PalletLocation :type "Vector Structure") (TargetPayload :type "Actor Object Reference"))
  (bind _targetlocation_location (`KismetMathLibrary.BreakTransform` (`self.TargetLocation`)))
  ;[1 1 1] legacy
  (bind _res (`self.PrePick`))
  (if _res
    (`self.SetPickTarget` PalletLocation TargetPayload)
    (`self.FindPickTargetpPyloadAndReachingPointEvent` _targetlocation_location (`self.TargetPayload`))
    (if (`self.FindTargetpayload`)
      (`self.PickImplEvent` (`self.ReachingPoint`)))))

(event `PickBTEvent`
  (params (PalletLocation :type "Vector Structure") (TargetPayload :type "Actor Object Reference") (UseApproach :type Boolean) (ApproachLocation :type "Vector Structure") (ApproachLocationActor :type "Actor Object Reference") (UseDefaultApproach :type Boolean))
  (bind _res (`self.PrePick`))
  (if _res
    (`self.SetPickTarget` PalletLocation TargetPayload UseApproach ApproachLocation ApproachLocationActor UseDefaultApproach)
    (set `self.BTTask` "NewEnumerator0")))

(event `PickImplEvent`
  (params (ReachintPoint :type "Transform Structure"))
  (bind (_returnvalue_x _returnvalue_y _returnvalue_z) (`KismetMathLibrary.BreakVector` (`self.K2_GetActorLocation`)))
  (bind _location (.location ReachintPoint))
  (bind _returnvalue (`self.K2_GetPawn`))
  ;[1 1 1] legacy
  (`|AIMoveTo` _returnvalue _location null 5.0 true
    (:`OnSuccess`
      (`self.LinearMoveToLocationWithDelegates` _returnvalue (`KismetMathLibrary.MakeVector` (.x _location) (.y _location) _returnvalue_z) (`KismetMathLibrary.MakeRotator` (.roll (.rotation ReachintPoint)) (.pitch (.rotation ReachintPoint)) (+ (.yaw (.rotation ReachintPoint)) 180.0)) (delegate `CustomEvent_5`) (delegate `CustomEvent_6`) 1.0 1.0 2.0 (0.0 0.0 0.0) (`KismetMathLibrary.MakeRotator` 0.0)))
    (:`OnFail`
      (`self.PostPick` false))))

(event `CustomEvent_3`
  ;[1 1 1] legacy
  (`self.AddLocalLinearMotionOffsetWthDelegates` (`self.K2_GetPawn`) (`KismetMathLibrary.MakeVector` (`/RapyutaSimulationPlugins/AI/BP_PickDropParam.DisToTarget` (`self.PickDropParam`))) (delegate `CustomEvent_1`) (delegate `CustomEvent_2`) :!label _label_3))

(event `CustomEvent_4`
  ;[1 1 1] legacy
  (`self.PostPick` false))

(event `CustomEvent_1`
  (bind (_returnvalue_x _returnvalue_y _returnvalue_z) (`KismetMathLibrary.BreakVector` (`self.K2_GetActorLocation`)))
  (bind (_returnvalue_x_2 _returnvalue_y_2 _returnvalue_z_2) (`KismetMathLibrary.BreakVector` (`self.K2_GetActorLocation` (`self.TargetPayload`))))
  (bind _attachmentjoint (`/RapyutaSimulationPlugins/AI/BP_PickDropParam.AttachmentJoint` (`self.PickDropParam`)))
  ;[1 1 1] legacy
  (`self.K2_AttachToComponent` (`self.TargetPayload`) (`/RapyutaSimulationPlugins/AI/BP_PickDropParam.AttachmentLink` (`self.PickDropParam`)) "None" "KeepWorld" "KeepWorld" "KeepWorld" true)
  (`/Engine/EditorBlueprintResources/StandardMacros.IsValid` _attachmentjoint
    (:`Is Valid`
      (`RRJointComponent.SetSinglePositionTargetWithDelegates` _attachmentjoint (- (+ _returnvalue_z_2 (`/RapyutaSimulationPlugins/AI/BP_PickDropParam.PickOffset` (`self.PickDropParam`))) _returnvalue_z) (delegate `CustomEvent_0`) (delegate `CustomEvent`) -1.0 5.0))
    (:`Is Not Valid`
      (`self.AddLocalLinearMotionOffsetWthDelegates` (`self.K2_GetPawn`) (`KismetMathLibrary.MakeVector` (* (`/RapyutaSimulationPlugins/AI/BP_PickDropParam.DisToTarget` (`self.PickDropParam`)) -1.0)) (delegate `CustomEvent_10`) (delegate `CustomEvent_9`) :!label _label_4))))

(event `CustomEvent_2`
  ;[1 1 1] legacy
  (`self.PostPick` false))

(event `CustomEvent_5`
  (bind (_returnvalue_x _returnvalue_y _returnvalue_z) (`KismetMathLibrary.BreakVector` (`self.K2_GetActorLocation`)))
  (bind (_returnvalue_x_2 _returnvalue_y_2 _returnvalue_z_2) (`KismetMathLibrary.BreakVector` (`self.K2_GetActorLocation` (`self.TargetPayload`))))
  (bind _attachmentjoint (`/RapyutaSimulationPlugins/AI/BP_PickDropParam.AttachmentJoint` (`self.PickDropParam`)))
  ;[1 1 1] legacy
  (`/Engine/EditorBlueprintResources/StandardMacros.IsValid` _attachmentjoint
    (:`Is Valid`
      (`RRJointComponent.SetSinglePositionTargetWithDelegates` _attachmentjoint (- _returnvalue_z_2 _returnvalue_z) (delegate `CustomEvent_3`) (delegate `CustomEvent_4`) -1.0 5.0))
    (:`Is Not Valid`
      (goto _label_3))))

(event `CustomEvent_6`
  ;[1 1 1] legacy
  (`self.PostPick` false))

(event `CustomEvent_10`
  ;[1 1 1] legacy
  (`self.PostPick` true))

(event `CustomEvent_9`
  ;[1 1 1] legacy
  (`self.PostPick` false))

(event `CustomEvent`
  ;[1 1 1] legacy
  (`self.PostPick` false))

(event `CustomEvent_0`
  ;[1 1 1] legacy
  (goto _label_4))

(event `PickSubCB`
  (params (InMessage :type "ROS2GenericMsg Object Reference"))
  (bind _output (`ROS2PointStampedMsg.GetMsg` (cast `ROS2PointStampedMsg` InMessage :!pure true)))
  (bind _returnvalue (`RRConversionUtils.TransformROSToUE` (`KismetMathLibrary.MakeTransform` (`.Point` (break `ROSPointStamped` _output)))))
  (bind _returnvalue_2 (`RRGeneralUtils.GetWorldTransformFromName` (`.FrameId` (break `ROSHeader` (break `ROSPointStamped` _output))) _returnvalue true))
  (`self.PickBTEvent` (.location _returnvalue_2) null (`self.UseApproach`) (`self.ApproachLocation`) null (`self.UseDefaultApproach`)))

(event `PickActorSubCB`
  (params (InMessage :type "ROS2GenericMsg Object Reference"))
  (bind _output_data (break `ROSStr` (`ROS2StrMsg.GetMsg` (cast `ROS2StrMsg` InMessage :!pure true))))
  (bind _returnvalue (`RRGeneralUtils.FindActorByName` _output_data))
  (`/Engine/EditorBlueprintResources/StandardMacros.IsValid` _returnvalue
    (:`Is Valid`
      (`self.PickBTEvent` (0.0 0.0 0.0) _returnvalue (`self.UseApproach`) (`self.ApproachLocation`) null (`self.UseDefaultApproach`)))
    (:`Is Not Valid`
      (`/RapyutaSimulationPlugins/Tools/RRGeneralUtility.DebugNamed Log` (`KismetStringLibrary.Concat_StrStr` "Can't find Actor named: " _output_data) self true true (struct :`R` 1.0 :`A` 1.0) 10.0 "None" (`self.Debug`)))))

(event `DropSubCB`
  (params (InMessage :type "ROS2GenericMsg Object Reference"))
  (bind _output (`ROS2PoseStampedMsg.GetMsg` (cast `ROS2PoseStampedMsg` InMessage :!pure true)))
  (bind _returnvalue (`RRConversionUtils.TransformROSToUE` (`KismetMathLibrary.MakeTransform` (break `ROSPose` (`.Pose` (break `ROSPoseStamped` _output))) (`KismetMathLibrary.Quat_Rotator` (`.Orientation` (break `ROSPose` (`.Pose` (break `ROSPoseStamped` _output))))))))
  (bind _returnvalue_2 (`RRGeneralUtils.GetWorldTransformFromName` (`.FrameId` (break `ROSHeader` (break `ROSPoseStamped` _output))) _returnvalue true))
  (`self.DropBTEvent` _returnvalue_2 null (`self.UseApproach`) (`self.ApproachLocation`) null (`self.UseDefaultApproach`)))

(event `DropActorSubCB`
  (params (InMessage :type "ROS2GenericMsg Object Reference"))
  (bind _output_data (break `ROSStr` (`ROS2StrMsg.GetMsg` (cast `ROS2StrMsg` InMessage :!pure true))))
  (bind _returnvalue (`RRGeneralUtils.FindActorByName` _output_data))
  (`/Engine/EditorBlueprintResources/StandardMacros.IsValid` _returnvalue
    (:`Is Valid`
      (`self.DropBTEvent` (struct) _returnvalue (`self.UseApproach`) (`self.ApproachLocation`) null (`self.UseDefaultApproach`)))
    (:`Is Not Valid`
      (`/RapyutaSimulationPlugins/Tools/RRGeneralUtility.DebugNamed Log` (`KismetStringLibrary.Concat_StrStr` "Can't find Actor named: " _output_data) self true true (struct :`R` 1.0 :`A` 1.0) 10.0 "None" (`self.Debug`)))))

(event `CustomEvent_19`
  (params (InMessage :type "ROS2GenericMsg Object Reference"))
  (bind _output (`ROS2PointStampedMsg.GetMsg` (cast `ROS2PointStampedMsg` InMessage :!pure true)))
  (bind _returnvalue (`RRConversionUtils.TransformROSToUE` (`KismetMathLibrary.MakeTransform` (`.Point` (break `ROSPointStamped` _output)))))
  (bind _returnvalue_2 (`RRGeneralUtils.GetWorldTransformFromName` (`.FrameId` (break `ROSHeader` (break `ROSPointStamped` _output))) _returnvalue true))
  (set `self.UseApproach` true)
  (set `self.ApproachLocation` (.location _returnvalue_2)))

(event `SetApproachLocationActorCB`
  (params (InMessage :type "ROS2GenericMsg Object Reference"))
  (bind _output_data (break `ROSStr` (`ROS2StrMsg.GetMsg` (cast `ROS2StrMsg` InMessage :!pure true))))
  (bind _returnvalue (`RRGeneralUtils.FindActorByName` _output_data))
  (`/Engine/EditorBlueprintResources/StandardMacros.IsValid` _returnvalue
    (:`Is Valid`
      (set `self.UseApproach` true)
      (set `self.ApproachLocation` (`self.K2_GetActorLocation` _returnvalue)))
    (:`Is Not Valid`
      (`/RapyutaSimulationPlugins/Tools/RRGeneralUtility.DebugNamed Log` (`KismetStringLibrary.Concat_StrStr` "Can't find Actor named: " _output_data) self true true (struct :`R` 1.0 :`A` 1.0) 10.0 "None" (`self.Debug`)))))

(event `CustomEvent_20`
  (params (InMessage :type "ROS2GenericMsg Object Reference"))
  (bind _output_bdata (break `ROSBool` (`ROS2BoolMsg.GetMsg` (cast `ROS2BoolMsg` InMessage :!pure true))))
  (set `self.UseDefaultApproach` _output_bdata)
  (set `self.UseApproach` true))

(event `TaskStatusPubCb`
  (params (InTopicMessage :type "ROS2GenericMsg Object Reference"))
  (`ROS2Int32Msg.SetMsg` (cast `ROS2Int32Msg` InTopicMessage :!pure true) (make `ROSInt32` (`KismetMathLibrary.Conv_ByteToInt` (`self.BTTask`)))))

(event `CustomEvent_21`
  (params (InMessage :type "ROS2GenericMsg Object Reference"))
  (bind _output_data (break `ROSStr` (`ROS2StrMsg.GetMsg` (cast `ROS2StrMsg` InMessage :!pure true))))
  (bind (_outjsonobject _returnvalue) (`JsonBlueprintFunctionLibrary.FromString` _output_data))
  (if _returnvalue
    (`self.GeneralAction` _outjsonobject)))

(event `self.BPInitROS2InterfaceImpl`
  (bind _dropsubscriber (`self.DropSubscriber`))
  (bind _picksubscriber (`self.PickSubscriber`))
  (bind _pickactorsubscriber (`self.PickActorSubscriber`))
  (bind _setapproachlocationsubscriber (`self.SetApproachLocationSubscriber`))
  (bind _dropactorsubscriber (`self.DropActorSubscriber`))
  (bind _setapproachlocationactorsubscriber (`self.SetApproachLocationActorSubscriber`))
  (bind _taskstatuspublisher (`self.TaskStatusPublisher`))
  (bind _setusedefaultapproachhsubscriber (`self.SetUseDefaultApproachhSubscriber`))
  (bind _generalactionsubscriber (`self.GeneralActionSubscriber`))
  (bind _subscriber (`ROS2SubscriberComponent.Subscriber` _dropsubscriber))
  (bind _subscriber_2 (`ROS2SubscriberComponent.Subscriber` _picksubscriber))
  (bind _subscriber_3 (`ROS2SubscriberComponent.Subscriber` _setapproachlocationsubscriber))
  (bind _subscriber_4 (`ROS2SubscriberComponent.Subscriber` _generalactionsubscriber))
  (bind _subscriber_5 (`ROS2SubscriberComponent.Subscriber` _pickactorsubscriber))
  (bind _subscriber_6 (`ROS2SubscriberComponent.Subscriber` _setapproachlocationactorsubscriber))
  (bind _subscriber_7 (`ROS2SubscriberComponent.Subscriber` _dropactorsubscriber))
  (bind _publisher (`ROS2PublisherComponent.Publisher` _taskstatuspublisher))
  (bind _subscriber_8 (`ROS2SubscriberComponent.Subscriber` _setusedefaultapproachhsubscriber))
  (`|ExecutionSequence`
    (:`then_0`
      (`|ExecutionSequence`
        (:`then_0`
          (`ROS2SubscriberComponent.DefaultCreateSubscriber` _picksubscriber)
          (`ROS2Subscriber.SetDelegates` _subscriber_2 (delegate `PickSubCB`))
          (`ROS2NodeComponent.AddSubscription` (`RRBaseROS2Interface.RobotROS2Node` (`self.ROS2Interface`)) _subscriber_2))
        (:`then_1`
          (`ROS2SubscriberComponent.DefaultCreateSubscriber` _pickactorsubscriber)
          (`ROS2Subscriber.SetDelegates` _subscriber_5 (delegate `PickActorSubCB`))
          (`ROS2NodeComponent.AddSubscription` (`RRBaseROS2Interface.RobotROS2Node` (`self.ROS2Interface`)) _subscriber_5))))
    (:`then_1`
      (`|ExecutionSequence`
        (:`then_0`
          (`|ExecutionSequence`
            (:`then_0`
              (`ROS2SubscriberComponent.DefaultCreateSubscriber` _dropsubscriber)
              (`ROS2Subscriber.SetDelegates` _subscriber (delegate `DropSubCB`))
              (`ROS2NodeComponent.AddSubscription` (`RRBaseROS2Interface.RobotROS2Node` (`self.ROS2Interface`)) _subscriber))
            (:`then_1`
              (`ROS2SubscriberComponent.DefaultCreateSubscriber` _dropactorsubscriber)
              (`ROS2Subscriber.SetDelegates` _subscriber_7 (delegate `DropActorSubCB`))
              (`ROS2NodeComponent.AddSubscription` (`RRBaseROS2Interface.RobotROS2Node` (`self.ROS2Interface`)) _subscriber_7))))
        (:`then_1`
          (`|ExecutionSequence`
            (:`then_0`
              (`|ExecutionSequence`
                (:`then_0`
                  (`ROS2SubscriberComponent.DefaultCreateSubscriber` _setapproachlocationsubscriber)
                  (`ROS2Subscriber.SetDelegates` _subscriber_3 (delegate `CustomEvent_19`))
                  (`ROS2NodeComponent.AddSubscription` (`RRBaseROS2Interface.RobotROS2Node` (`self.ROS2Interface`)) _subscriber_3))
                (:`then_1`
                  (`ROS2SubscriberComponent.DefaultCreateSubscriber` _setapproachlocationactorsubscriber)
                  (`ROS2Subscriber.SetDelegates` _subscriber_6 (delegate `SetApproachLocationActorCB`))
                  (`ROS2NodeComponent.AddSubscription` (`RRBaseROS2Interface.RobotROS2Node` (`self.ROS2Interface`)) _subscriber_6))))
            (:`then_1`
              (`|ExecutionSequence`
                (:`then_0`
                  (`|ExecutionSequence`
                    (:`then_0`
                      (`ROS2SubscriberComponent.DefaultCreateSubscriber` _setusedefaultapproachhsubscriber)
                      (`ROS2Subscriber.SetDelegates` _subscriber_8 (delegate `CustomEvent_20`))
                      (`ROS2NodeComponent.AddSubscription` (`RRBaseROS2Interface.RobotROS2Node` (`self.ROS2Interface`)) _subscriber_8))
                    (:`then_1`
                      (`ROS2PublisherComponent.DefaultCreatePublisher` _taskstatuspublisher)
                      (`ROS2Publisher.SetDelegates` _publisher (delegate `TaskStatusPubCb`))
                      (`ROS2NodeComponent.AddPublisher` (`RRBaseROS2Interface.RobotROS2Node` (`self.ROS2Interface`)) _publisher))))
                (:`then_1`
                  (`ROS2SubscriberComponent.DefaultCreateSubscriber` _generalactionsubscriber)
                  (`ROS2Subscriber.SetDelegates` _subscriber_4 (delegate `CustomEvent_21`))
                  (`ROS2NodeComponent.AddSubscription` (`RRBaseROS2Interface.RobotROS2Node` (`self.ROS2Interface`)) _subscriber_4))))))))))

(fn `BehaviorTreeSetting`
  (bind _pickdropparam (`self.PickDropParam`))
  (bind _asbehavior_tree_component (cast `BehaviorTreeComponent` (`self.BrainComponent`) :!pure true))
  (`self.RunBehaviorTree` "/RapyutaSimulationPlugins/AI/BT_ROS2Agent.BT_ROS2Agent")
  (`BehaviorTreeComponent.SetDynamicSubtree` _asbehavior_tree_component (struct :`TagName` "PickImpl") (`/RapyutaSimulationPlugins/AI/BP_PickDropParam.PickImplBehavior` _pickdropparam))
  (`BehaviorTreeComponent.SetDynamicSubtree` _asbehavior_tree_component (struct :`TagName` "DropImpl") (`/RapyutaSimulationPlugins/AI/BP_PickDropParam.DropImplBehavior` _pickdropparam)))

(fn `Find Pick Reaching Point`
  (params (`Target Pose` :type "Vector Structure") (`Target Actor` :type "Actor Object Reference"))
  (returns (ReachingPoint :type "Transform Structure") (Res :type Boolean))
  (bind _pickdropparam (`self.PickDropParam`))
  (`/Engine/EditorBlueprintResources/StandardMacros.IsValid` `Target Actor`
    (:`Is Valid`
      (set `self.TargetPayload` `Target Actor`))
    (:`Is Not Valid`
      (bind _newparam (`/RapyutaSimulationPlugins/Tools/RRGeneralUtility.Find Actor WIth Tag In Threshold` `Target Pose` (100.0 100.0 100.0) "Payload" `Target Actor`))
      (`/Engine/EditorBlueprintResources/StandardMacros.IsValid` _newparam
        (:`Is Valid`
          (set `self.TargetPayload` _newparam))
        (:`Is Not Valid`
          (return (struct) false)))))
  (bind _closestreachingpoint (`/RapyutaSimulationPlugins/Tools/RRGeneralUtility.Find Reaching Point` (`self.GetTransform` (`self.TargetPayload`)) (+ (`/RapyutaSimulationPlugins/AI/BP_PickDropParam.ReachingOffset` _pickdropparam) (`/RapyutaSimulationPlugins/AI/BP_PickDropParam.DisToTarget` _pickdropparam)) self))
  (bind _output_get (set `self.ReachingPoint` _closestreachingpoint))
  (return _output_get true))

(fn `FindDropReachingPoint`
  (params (TargetLocation :type "Transform Structure"))
  (returns (Output_Get :type "Transform Structure"))
  (locals (tempTargetLocation :type "Transform Structure"))
  (bind _pickdropparam (`self.PickDropParam`))
  (bind _closestreachingpoint (`/RapyutaSimulationPlugins/Tools/RRGeneralUtility.Find Reaching Point` TargetLocation (+ (`/RapyutaSimulationPlugins/AI/BP_PickDropParam.ReachingOffset` _pickdropparam) (`/RapyutaSimulationPlugins/AI/BP_PickDropParam.DisToTarget` _pickdropparam)) (`self.K2_GetPawn` self)))
  (bind _output_get (set `self.ReachingPoint` _closestreachingpoint))
  (return _output_get))

(fn `GeneralAction`
  (params (JsonParam :type "JsonObjectWrapper Structure"))
  (if (`|EnumEquality` (`self.BTTask`) "NewEnumerator2")
    (bind _asbp_rraibase_robot (cast `/RapyutaSimulationPlugins/Robots/BP_RRAIBaseRobot` (`self.K2_GetPawn`)))
    (`/RapyutaSimulationPlugins/Robots/BP_RRAIBaseRobot.GeneralAction` _asbp_rraibase_robot JsonParam)))

(fn `PostDrop`
  (params (res :type Boolean))
  (set `self.IsTaskProcessing` false)
  (set `self.IsCarrying` (not res))
  (set `self.UseApproach` false)
  (`/RapyutaSimulationPlugins/AI/BP_PickDropParam.CopyParam` (`self.PickDropParam`) (`self.DefaultPickDropParam`)))

(fn `PostPick`
  (params (res :type Boolean))
  (set `self.IsTaskProcessing` false)
  (set `self.IsCarrying` res)
  (set `self.UseApproach` false))

(fn `PreDrop`
  (returns (Res :type Boolean))
  ;[1 1 1] Check before start
  (if (`self.IsTaskProcessing`)
    (`KismetSystemLibrary.PrintString` "Still processing last request" true true (struct :`R` 1.0 :`B` 0.047707 :`A` 1.0) 200.0)
    (elif (`self.IsCarrying`)
      (return true)
      (else
        (`KismetSystemLibrary.PrintString` "Not carrying payload" true true (struct :`R` 1.0 :`G` 0.056108 :`A` 1.0) 200.0))))
  (return false))

(fn `PrePick`
  (returns (Res :type Boolean))
  ;[1 1 1] Check before start
  (if (`self.IsTaskProcessing`)
    (`KismetSystemLibrary.PrintString` "Still processing last request" true true (struct :`R` 1.0 :`B` 0.047707 :`A` 1.0) 200.0)
    (elif (`self.IsCarrying`)
      (`KismetSystemLibrary.PrintString` "Already carrying payload" true true (struct :`R` 1.0 :`G` 0.056108 :`A` 1.0) 200.0)
      (else
        (return true))))
  (return false))

(fn `SetDropTarget`
  (params (TargetLocation :type "Transform Structure") (TargetLocationActor :type "Actor Object Reference") (UseApproach :type Boolean) (ApproachLocation :type "Vector Structure") (ApproachLocationActor :type "Actor Object Reference") (UseDefaultApproach :type Boolean))
  (returns (OutLocation :type "Transform Structure"))
  (bind _returnvalue (`self.GetParentActor` TargetLocationActor))
  (bind _returnvalue_2 (`self.GetAttachParentActor` TargetLocationActor))
  (set `self.DropTargetParent` null)
  (set `self.UseDefaultApproach` UseDefaultApproach)
  (bind _output_get (set `self.UseApproach` UseApproach))
  (if _output_get
    (bind _approachpoint (`/RapyutaSimulationPlugins/Tools/RRGeneralUtility.GetApproachPointFromChildOfPayloadBase` TargetLocationActor))
    (if (and (`KismetSystemLibrary.IsValid` _approachpoint) UseDefaultApproach)
      (set `self.ApproachLocation` (`self.K2_GetActorLocation` _approachpoint))
      (else
        (`/Engine/EditorBlueprintResources/StandardMacros.IsValid` ApproachLocationActor
          (:`Is Valid`
            (set `self.ApproachLocation` (`self.K2_GetActorLocation` ApproachLocationActor)))
          (:`Is Not Valid`
            (set `self.ApproachLocation` ApproachLocation))))))
  (`/Engine/EditorBlueprintResources/StandardMacros.IsValid` TargetLocationActor
    (:`Is Valid`
      (`/Engine/EditorBlueprintResources/StandardMacros.IsValid` _returnvalue
        (:`Is Valid`
          (set `self.DropTargetParent` _returnvalue))
        (:`Is Not Valid`
          (`/Engine/EditorBlueprintResources/StandardMacros.IsValid` _returnvalue_2
            (:`Is Valid`
              (set `self.DropTargetParent` _returnvalue_2))
            (:`Is Not Valid`
              _))))
      (bind _output_get_2 (set `self.TargetLocation` (`self.GetTransform` TargetLocationActor)))
      (return _output_get_2))
    (:`Is Not Valid`
      (bind _output_get_3 (set `self.TargetLocation` TargetLocation))
      (return _output_get_3))))

(fn `SetPickTarget`
  (params (TargetLocation :type "Vector Structure") (TargetPayloadActor :type "Actor Object Reference") (UseApproach :type Boolean) (ApproachLocation :type "Vector Structure") (ApproachLocationActor :type "Actor Object Reference") (UseDefaultApproach :type Boolean))
  (returns (OutLocation :type "Vector Structure") (OutActor :type "Actor Object Reference"))
  (set `self.UseDefaultApproach` UseDefaultApproach)
  (bind _output_get (set `self.UseApproach` UseApproach))
  (if _output_get
    (`/Engine/EditorBlueprintResources/StandardMacros.IsValid` ApproachLocationActor
      (:`Is Valid`
        (set `self.ApproachLocation` (`self.K2_GetActorLocation` ApproachLocationActor)))
      (:`Is Not Valid`
        (set `self.ApproachLocation` ApproachLocation))))
  (`/Engine/EditorBlueprintResources/StandardMacros.IsValid` TargetPayloadActor
    (:`Is Valid`
      (bind _output_get_2 (set `self.TargetPayload` TargetPayloadActor))
      (return (0.0 0.0 0.0) _output_get_2))
    (:`Is Not Valid`
      (bind _output_get_3 (set `self.TargetLocation` (`KismetMathLibrary.MakeTransform` TargetLocation)))
      (return (.location _output_get_3) null))))

(fn `UserConstructionScript`)